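; BP_Obs_Cube2 is an endless runner obstacle with two trigger boxes, Box1 and Box2, that detect the player's BP_Runner.
; On begin overlap with either box, it calls HitObstacleMessage on the runner only if the runner's IsOffObs flag is true.
; On end overlap it sets IsOffObs to true; this graph never clears the flag.
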(event OnComponentBeginOverlap(Box2)
  (params (OverlappedComponent :type Primitive%20Component%20Object%20Reference) (OtherActor :type Actor%20Object%20Reference) (OtherComp :type Primitive%20Component%20Object%20Reference) (OtherBodyIndex :type Integer) (bFromSweep :type Boolean) (SweepResult :type Hit%20Result%20Structure%20%28by%20ref%29))
  (bind _asbp_runner (Utilities|Casting|CastToBP_Runner OtherActor))
  (if (Variables|/Game/Endless_Runner/Blueprints/BluePrint/BP_Runner.BP_Runner_C|GetisOffObs _asbp_runner)
    (Class|BPInterface|HitObstacle(Message) _asbp_runner)))

(event OnComponentEndOverlap(Box1)
  (params (OverlappedComponent :type Primitive%20Component%20Object%20Reference) (OtherActor :type Actor%20Object%20Reference) (OtherComp :type Primitive%20Component%20Object%20Reference) (OtherBodyIndex :type Integer))
  (bind _asbp_runner (Utilities|Casting|CastToBP_Runner OtherActor))
  (Variables|/Game/Endless_Runner/Blueprints/BluePrint/BP_Runner.BP_Runner_C|SetisOffObs _asbp_runner true))

(event OnComponentBeginOverlap(Box1)
  (params (OverlappedComponent :type Primitive%20Component%20Object%20Reference) (OtherActor :type Actor%20Object%20Reference) (OtherComp :type Primitive%20Component%20Object%20Reference) (OtherBodyIndex :type Integer) (bFromSweep :type Boolean) (SweepResult :type Hit%20Result%20Structure%20%28by%20ref%29))
  (bind _asbp_runner (Utilities|Casting|CastToBP_Runner OtherActor))
  (if (Variables|/Game/Endless_Runner/Blueprints/BluePrint/BP_Runner.BP_Runner_C|GetisOffObs _asbp_runner)
    (Class|BPInterface|HitObstacle(Message) _asbp_runner)))

(event OnComponentEndOverlap(Box2)
  (params (OverlappedComponent :type Primitive%20Component%20Object%20Reference) (OtherActor :type Actor%20Object%20Reference) (OtherComp :type Primitive%20Component%20Object%20Reference) (OtherBodyIndex :type Integer))
  (bind _asbp_runner (Utilities|Casting|CastToBP_Runner OtherActor))
  (Variables|/Game/Endless_Runner/Blueprints/BluePrint/BP_Runner.BP_Runner_C|SetisOffObs _asbp_runner true))

(event EventBeginPlay)

(event Collision|EventActorBeginOverlap
  (params (OtherActor :type Actor%20Object%20Reference)))

(event EventTick
  (params (DeltaSeconds :type Float%20%28single-precision%29)))

(fn ConstructionScript
  (|CallParentFunction))