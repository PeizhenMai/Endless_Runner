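; BP_Floor is a floor tile for an endless runner that triggers track generation when the runner touches it.
; On overlap with BP_Runner, it asks the runner to generate the next floor at its Arrow transform, plus obstacles and pickups based on the player's position.
; Five seconds later it clears its IsInUse flag, and GetArrowTransform exposes the Arrow's world transform.
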(event OnComponentBeginOverlap(floor)
  (params (OverlappedComponent :type Primitive%20Component%20Object%20Reference) (OtherActor :type Actor%20Object%20Reference) (OtherComp :type Primitive%20Component%20Object%20Reference) (OtherBodyIndex :type Integer) (bFromSweep :type Boolean) (SweepResult :type Hit%20Result%20Structure%20%28by%20ref%29))
  (bind _returnvalue (Game|GetPlayerCharacter 0))
  (bind _returnvalue_2 (Transformation|GetActorTransform _returnvalue))
  (bind _asbp_runner (Utilities|Casting|CastToBP_Runner OtherActor))
  (Default|GenerateFloor _asbp_runner (Transformation|GetWorldTransform (Variables|Default|GetArrow)))
  (Default|GenerateObstacle _asbp_runner (Math|Transform|MakeTransform (Math|Vector|MakeVector (.x (.location _returnvalue_2)) 0.0 (.z (.location _returnvalue_2))) "0, 0, 0" "1.000000,1.000000,1.000000"))
  (Default|GeneratePickup _asbp_runner (Transformation|GetActorTransform _returnvalue))
  (Utilities|FlowControl|Delay 5.0)
  (Variables|Default|SetIs%20in%20Use? false))

(fn ConstructionScript)

(fn GetArrowTransform
  (return (Transformation|GetWorldTransform (Variables|Default|GetArrow))))