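; Game instance Blueprint for the endless runner that provides functions to obfuscate and restore name strings.
; ObfsName follows each character of the name with four random picks from a junk-letter array.
; UnObfsName reverses this by keeping the first character of every group of five, so it is simple padding with no key.
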(fn ObfsName
  (params (Unaltered%20Name :type String))
  (for _array_element (Utilities|String|GetCharacterArrayfromString Unaltered%20Name)
    (LocalVariables|SetFinalString (Utilities|String|Append (LocalVariables|GetFinalString) _array_element))
    (for _index (range 0 3)
      (LocalVariables|SetFinalString (Utilities|String|Append (LocalVariables|GetFinalString) (Utilities|Array|Get(acopy) (Variables|Default|GetArrayofJunkLetter) (Math|Random|RandomIntegerinRange 0 7))))))
  (return (LocalVariables|GetFinalString)))

(fn UnObfsName
  (params (Obfs%20Name :type String))
  (for _array_element (Utilities|String|GetCharacterArrayfromString Obfs%20Name)
    (if (== (LocalVariables|GetCount) 0)
      (LocalVariables|SetNewString (Utilities|String|Append (LocalVariables|GetNewString) _array_element)))
    (Math|Integer|IncrementInt (LocalVariables|GetCount)
      (:%20%20
        (if (> (LocalVariables|GetCount) 4)
          (LocalVariables|SetCount 0)))))
  (return (LocalVariables|GetNewString)))