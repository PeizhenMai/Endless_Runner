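; Game mode for an endless runner that tracks the current score and the persistent high score.
; On BeginPlay it loads the high score from an SG_HighScore save slot.
; Every Tick it caps the Capsule count and BP_Runner's walk speed, writes a save whenever the score beats the record, and copies the score to Endless_GameInstance.
; GeneratePickup and TimeSlow are empty stubs.
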(event EventBeginPlay
  (bind _returnvalue (SaveGame|DoesSaveGameExist "HighScoreSlot"))
  (if _returnvalue
    (bind _returnvalue_2 (SaveGame|LoadGamefromSlot "HighScoreSlot"))
    (bind _assg_high_score (Utilities|Casting|CastToSG_HighScore _returnvalue_2))
    (Variables|Default|SetHighScore (Variables|/Game/Endless_Runner/SaveGame/SG_HighScore.SG_HighScore_C|GetHistoryHighScore _assg_high_score))))

(event EventTick
  (params (DeltaSeconds :type Float%20%28single-precision%29))
  (Utilities|FlowControl|Sequence
    (:then_0
      (|MaxCapsule))
    (:then_1
      (|MaxWalkSpeed))
    (:then_2
      (|SaveHighScore))
    (:then_3
      (|SetScoreToGameInstace))))

(fn ConstructionScript)

(fn GeneratePickup)

(fn TimeSlow)